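; BP_Sparrow is the Sparrow enemy AI, handling player sight and a gust attack.
; PawnSensing sets a "seen player" Blackboard key when it spots the third-person character, and a retriggerable delay clears it after a few seconds without a sighting.
; GustAttack sphere-traces a short distance ahead for pawns with debug drawing on, and plays the attack montage if it hits the player, applying no damage here.
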(event OnSeePawn(PawnSensing)
  (params (Pawn :type Pawn%20Object%20Reference))
  ;[1 1 1] Sparrow Sight
  ;;[0 1 0.00595] Sees player and turns variable on
  (Utilities|Casting|CastToBP_ThirdPersonCharacter Pawn)
  (Utilities|FlowControl|Sequence
    (:then_0
      (bind _output_get (Variables|Default|SetcanSeePlayer? true))
      (AI|Components|Blackboard|SetValueasBool (AI|GetBlackboard (AI|GetAIController self)) (Utilities|Name|MakeLiteralName "hasSeenPlayer?") _output_get))
    (:then_1
      (Utilities|FlowControl|RetriggerableDelay 5.0)
      (bind _output_get_2 (Variables|Default|SetcanSeePlayer? false))
      ;;[1 0 0.007267] Checks that player is no longer on sight
      (AI|Components|Blackboard|SetValueasBool (AI|GetBlackboard (AI|GetAIController self)) (Utilities|Name|MakeLiteralName "hasSeenPlayer?") _output_get_2))))

(event Custom|Gust%20Attack
  (bind _returnvalue (Transformation|GetActorLocation))
  (bind (_outhit _returnvalue_2) (Collision|SphereTraceForObjects _returnvalue (+ _returnvalue (* (Math|Vector|GetForwardVector (Transformation|GetActorRotation)) 2.5e+02)) 1.2e+02 (Utilities|Array|MakeArray "ObjectTypeQuery3") false 0 "ForDuration"))
  (if _returnvalue_2
    (Utilities|Casting|CastToBP_ThirdPersonCharacter (.HitActor (Collision|BreakHitResult _outhit)))
    (Animation|PlayAnimMontage "/Game/TeamOrange/Josh/Sparrow/textures/source/Mont_Sparrow_Attack.Mont_Sparrow_Attack" 1.0 "None")))

(event EventBeginPlay)

(event Collision|EventActorBeginOverlap
  (params (OtherActor :type Actor%20Object%20Reference)))

(event EventTick
  (params (DeltaSeconds :type Float%20%28single-precision%29)))

(fn ConstructionScript)